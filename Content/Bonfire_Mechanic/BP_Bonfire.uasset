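; Bonfire interactable actor that lets the player open a bonfire menu while standing nearby.
; Sphere overlap flags the character's stats component as in an upgrade zone, adds the bonfire input mapping context and enables input on the actor; leaving reverses all three.
; The interact action creates the menu widget, switches to UI-only input with a visible cursor and stops character movement.
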(event OnComponentBeginOverlap(Sphere)
  (params (OverlappedComponent :type Primitive%20Component%20Object%20Reference) (OtherActor :type Actor%20Object%20Reference) (OtherComp :type Primitive%20Component%20Object%20Reference) (OtherBodyIndex :type Integer) (bFromSweep :type Boolean) (SweepResult :type Hit%20Result%20Structure%20%28by%20ref%29))
  ;[0.15 0 0 0.5] On Begin Overlap
  (bind _asbp_third_person_character (Utilities|Casting|CastToBP_ThirdPersonCharacter OtherActor))
  (Variables|/Game/ThirdPerson/Blueprints/BPC_Stats.BPC_Stats_C|SetIsInUpgradeZone (Variables|/Game/ThirdPerson/Blueprints/BP_ThirdPersonCharacter.BP_ThirdPersonCharacter_C|GetBPC_Stats _asbp_third_person_character) true)
  (bind _asplayer_controller (Utilities|Casting|CastToPlayerController (Pawn|GetController _asbp_third_person_character)))
  (Input|AddMappingContext (PlayerController|LocalPlayerSubsystems|GetEnhancedInputLocalPlayerSubsystem _asplayer_controller) "/Game/Bonfire_Mechanic/IMC_Bonfire.IMC_Bonfire" 0 "(bIgnoreAllPressedKeysUntilRelease=True,bForceImmediately=False,bNotifyUserSettings=False)")
  (Input|EnableInput _asplayer_controller))

(event OnComponentEndOverlap(Sphere)
  (params (OverlappedComponent :type Primitive%20Component%20Object%20Reference) (OtherActor :type Actor%20Object%20Reference) (OtherComp :type Primitive%20Component%20Object%20Reference) (OtherBodyIndex :type Integer))
  ;[0 0.02119 0.15 0.5] End Begin Overlap
  (bind _asbp_third_person_character (Utilities|Casting|CastToBP_ThirdPersonCharacter OtherActor))
  (Variables|/Game/ThirdPerson/Blueprints/BPC_Stats.BPC_Stats_C|SetIsInUpgradeZone (Variables|/Game/ThirdPerson/Blueprints/BP_ThirdPersonCharacter.BP_ThirdPersonCharacter_C|GetBPC_Stats _asbp_third_person_character) false)
  (bind _asplayer_controller (Utilities|Casting|CastToPlayerController (Pawn|GetController _asbp_third_person_character)))
  (Input|RemoveMappingContext (PlayerController|LocalPlayerSubsystems|GetEnhancedInputLocalPlayerSubsystem _asplayer_controller) "/Game/Bonfire_Mechanic/IMC_Bonfire.IMC_Bonfire" "(bIgnoreAllPressedKeysUntilRelease=True,bForceImmediately=False,bNotifyUserSettings=False)")
  (Input|DisableInput _asplayer_controller))

(event Input|EnhancedActionEvents|EnhancedInputActionIA_UseInteractiveObject
  (params (ActionValue :type Boolean) (ElapsedSeconds :type Float%20%28double-precision%29) (TriggeredSeconds :type Float%20%28double-precision%29) (InputAction :type Input%20Action%20Object%20Reference :default "/Game/Bonfire_Mechanic/IA_UseInteractiveObject.IA_UseInteractiveObject"))
  (bind _returnvalue (Game|GetPlayerController 0))
  ;[0.15 0 0 0.5] Use Bonfire
  (:Started
    (bind _returnvalue_2 (UserInterface|CreateWidget "/Game/UI_Wİdgets/WB_BonfireMenu.WB_BonfireMenu_C"))
    (UserInterface|Viewport|AddtoViewport _returnvalue_2 0)
    (Input|SetInputModeUIOnly _returnvalue _returnvalue_2 "DoNotLock" false)
    (Variables|/Script/Engine.PlayerController|SetbShowMouseCursor _returnvalue true)
    (Pawn|Components|CharacterMovement|SetMovementMode (Variables|/Script/Engine.Character|GetCharacterMovement (Game|GetPlayerCharacter 0)) "MOVE_None" 0)))

(event EventBeginPlay)

(event Collision|EventActorBeginOverlap
  (params (OtherActor :type Actor%20Object%20Reference)))

(event EventTick
  (params (DeltaSeconds :type Float%20%28single-precision%29)))

(fn ConstructionScript)