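; BP_Aurora is a melee enemy character, with optional boss trace points, that damages the player and awards XP on death.
; A looping timer drives sword sphere traces with DoOnce-throttled damage, alongside a separate single-point attack trace.
; Incoming damage feeds BPCStats, linked to the health bar, and plays a movement-halting hit montage.
; Death ragdolls the body and clears player target lock, granting XP only if the lock widget exists.
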(event Custom|CustomEvent
  ;[0.15 0.15 0.15 0.5] Sword Traces
  (if (not (Variables|Default|GetIsDeath?))
    (bind (_outhit _returnvalue) (Collision|SphereTraceForObjects (Math|Vector|SelectVector (Variables|Default|GetBossStartSwordTrace) (Transformation|GetWorldLocation (Variables|Default|GetStartTraceAurora)) (Variables|Default|GetIsBoss?)) (Math|Vector|SelectVector (Variables|Default|GetBossEndSwordTrace) (Transformation|GetWorldLocation (Variables|Default|GetEndTraceAurora)) (Variables|Default|GetIsBoss?)) (Variables|Default|GetSwordAttackRadius) (Utilities|Array|MakeArray "ObjectTypeQuery3") false 0 "ForOneFrame"))
    ;;[0.15 0.15 0.15 0.5] Apply Damage
    (if _returnvalue
      (Utilities|FlowControl|DoOnce false :!label _label
        (:Completed
          (Game|Damage|ApplyDamage (.HitActor (Collision|BreakHitResult _outhit)) (Variables|Default|GetSword%20Damage) 0 0)
          (Utilities|FlowControl|Delay 0.3)
          (goto _label Reset))))))

(event EventPointDamageTrace
  (bind _pointtracepos (Variables|Default|GetPointTracePos))
  (bind _returnvalue (Transformation|GetWorldLocation _pointtracepos))
  ;[0.15 0.15 0.15 0.5] Damage Done
  (bind (_outhit _returnvalue_2) (Collision|SphereTraceForObjects _returnvalue _returnvalue (Variables|Default|GetPointAttackRadius) (Utilities|Array|MakeArray "ObjectTypeQuery3") false 0 "ForDuration"))
  (if _returnvalue_2
    (Game|Damage|ApplyDamage (.HitActor (Collision|BreakHitResult _outhit)) 15.0 0 0)))

(event EventEndSwordTrace
  ;[0.15 0.15 0.15 0.5] Sword Traces
  (if (Utilities|Time|IsValidTimerHandle (stale EventBeginSwordTrace _returnvalue))
    (Utilities|Time|ClearandInvalidateTimerbyHandle (stale EventBeginSwordTrace _returnvalue))))

(event EventBeginPlay
  ;[0.15 0.15 0.15 0.5] Widget
  (bind _asbp_third_person_character (Utilities|Casting|CastToBP_ThirdPersonCharacter (Game|GetPlayerCharacter 0)))
  (Variables|Default|SetPlayerRef _asbp_third_person_character)
  (bind _aswb_enemy_health_bar (Utilities|Casting|CastToWB_EnemyHealthBar (UserInterface|GetWidget (Variables|Default|GetHealthBar))))
  (Default|SetHealthProgressBar (Variables|Default|GetBPC_Stats) (Variables|/Game/UI_Wİdgets/WB_EnemyHealthBar.WB_EnemyHealthBar_C|GetHealthBar _aswb_enemy_health_bar)))

(event EventDeath
  (bind _playerref (Variables|Default|GetPlayerRef))
  (bind _capsulecomponent (Variables|Default|GetCapsuleComponent))
  (bind _playerref_2 (Variables|Default|GetPlayerRef))
  (bind _charactermovement (Variables|/Script/Engine.Character|GetCharacterMovement _playerref))
  (bind _bpc_combat (Variables|/Game/ThirdPerson/Blueprints/BP_ThirdPersonCharacter.BP_ThirdPersonCharacter_C|GetBPC_Combat _playerref_2))
  ;[0.15 0 0 0.5] Die
  (Class|Pawn|DetachfromControllerPendingDestroy)
  (Pawn|Components|CharacterMovement|DisableMovement (Variables|Character|GetCharacterMovement))
  (Physics|SetSimulatePhysics (Variables|Character|GetMesh) true)
  (Components|Animation|SetAnimationMode (Variables|Character|GetMesh) "AnimationSingleNode" true)
  (Variables|Default|SetIsDeath? true)
  (Collision|SetCollisionEnabled _capsulecomponent "NoCollision")
  (Collision|SetCollisionResponsetoChannel _capsulecomponent "ECC_Pawn" "ECR_Ignore")
  (Variables|/Game/ThirdPerson/Blueprints/BPC_Combat.BPC_Combat_C|SetTargetLockActor _bpc_combat 0)
  (Utilities|IsValid (Variables|/Game/ThirdPerson/Blueprints/BPC_Combat.BPC_Combat_C|GetTargetLockWB _bpc_combat)
    (:Is%20Valid
      (Default|AddXP (Variables|/Game/ThirdPerson/Blueprints/BP_ThirdPersonCharacter.BP_ThirdPersonCharacter_C|GetBPC_Stats _playerref_2) (Variables|Default|GetXPAward))
      (Actor|DestroyActor (Variables|/Game/ThirdPerson/Blueprints/BPC_Combat.BPC_Combat_C|GetTargetLockWB _bpc_combat)))
    (:Is%20Not%20Valid
      _))
  (Variables|/Game/ThirdPerson/Blueprints/BPC_Combat.BPC_Combat_C|SetTargetLockWB _bpc_combat (Variables|/Game/ThirdPerson/Blueprints/BPC_Combat.BPC_Combat_C|GetTargetLockWB _bpc_combat))
  (Variables|/Script/Engine.CharacterMovementComponent|SetbOrientRotationToMovement _charactermovement true)
  (Variables|/Script/Engine.CharacterMovementComponent|SetbUseControllerDesiredRotation _charactermovement false)
  (Rendering|SetVisibility (Variables|Default|GetHealthBar) false false))

(event Game|Damage|EventAnyDamage
  (params (Damage :type Float%20%28single-precision%29) (DamageType :type Damage%20Type%20Object%20Reference) (InstigatedBy :type Controller%20Object%20Reference) (DamageCauser :type Actor%20Object%20Reference))
  (bind _charactermovement (Variables|Character|GetCharacterMovement))
  ;[0.15 0.15 0.15 0.5] Damage Received
  (Default|IncreaseValue (Variables|Default|GetBPC_Stats) "NewEnumerator0" (* Damage -1.0))
  (Animation|Montage|PlayMontage (Variables|Character|GetMesh) "/Game/Dark_Knight/Dark_Knight_Female/Animations/Anim_DKF_Hit_Fwd_Montage.Anim_DKF_Hit_Fwd_Montage"
    (:then
      (Variables|/Script/Engine.CharacterMovementComponent|SetMaxWalkSpeed _charactermovement 0.0))
    (:OnCompleted
      (Variables|/Script/Engine.CharacterMovementComponent|SetMaxWalkSpeed _charactermovement 4.5e+02 :!label _label))
    (:OnInterrupted
      (goto _label))))

(event EventBeginSwordTrace
  ;[0.15 0.15 0.15 0.5] Sword Traces
  (bind _returnvalue (Utilities|Time|SetTimerbyEvent (delegate Custom|CustomEvent) 0.01 true)))

(fn ConstructionScript
  (|CallParentFunction))