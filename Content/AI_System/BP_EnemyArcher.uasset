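; BP_EnemyArcher is an enemy character that plays sword and hard attack montages and deals point damage through a sphere trace.
; Incoming damage lowers a BPCStats value and plays a hit montage that halts walking until it ends.
; BeginPlay binds the health bar widget to BPCStats and caches the player.
; Death ragdolls the mesh, disables capsule collision, hides the health bar and clears the player's target lock.
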(event EventPointDamageTrace
  (bind _pointtracepos (Variables|Default|GetPointTracePos))
  (bind _returnvalue (Transformation|GetWorldLocation _pointtracepos))
  ;[0.15 0.15 0.15 0.5] Damage Done
  (bind (_outhit _returnvalue_2) (Collision|SphereTraceForObjects _returnvalue _returnvalue (Variables|Default|GetPointAttackRadius) (Utilities|Array|MakeArray "ObjectTypeQuery3") false 0 "ForDuration"))
  (if _returnvalue_2
    (Game|Damage|ApplyDamage (.HitActor (Collision|BreakHitResult _outhit)) 1e+01 0 0)))

(event EventBeginPlay
  ;[0.15 0.15 0.15 0.5] Widget
  (bind _asbp_third_person_character (Utilities|Casting|CastToBP_ThirdPersonCharacter (Game|GetPlayerCharacter 0)))
  (Variables|Default|SetPlayerRef _asbp_third_person_character)
  (bind _aswb_enemy_health_bar (Utilities|Casting|CastToWB_EnemyHealthBar (UserInterface|GetWidget (Variables|Default|GetHealthBar))))
  (Default|SetHealthProgressBar (Variables|Default|GetBPC_Stats) (Variables|/Game/UI_Wİdgets/WB_EnemyHealthBar.WB_EnemyHealthBar_C|GetHealthBar _aswb_enemy_health_bar)))

(event EventDeath
  (bind _playerref (Variables|Default|GetPlayerRef))
  (bind _capsulecomponent (Variables|Collision|GetCapsuleComponent))
  (bind _playerref_2 (Variables|Default|GetPlayerRef))
  (bind _charactermovement (Variables|/Script/Engine.Character|GetCharacterMovement _playerref))
  (bind _bpc_combat (Variables|/Game/ThirdPerson/Blueprints/BP_ThirdPersonCharacter.BP_ThirdPersonCharacter_C|GetBPC_Combat _playerref_2))
  ;[0.15 0 0 0.5] Die
  (Pawn|Components|CharacterMovement|DisableMovement (Variables|Character|GetCharacterMovement))
  (Physics|SetSimulatePhysics (Variables|Character|GetMesh) true)
  (Variables|Default|SetIsDeath? true)
  (Collision|SetCollisionEnabled _capsulecomponent "NoCollision")
  (Collision|SetCollisionResponsetoChannel _capsulecomponent "ECC_Pawn" "ECR_Ignore")
  (Variables|/Game/ThirdPerson/Blueprints/BPC_Combat.BPC_Combat_C|SetTargetLockActor _bpc_combat 0)
  (Actor|DestroyActor (Variables|/Game/ThirdPerson/Blueprints/BPC_Combat.BPC_Combat_C|GetTargetLockWB _bpc_combat))
  (Variables|/Game/ThirdPerson/Blueprints/BPC_Combat.BPC_Combat_C|SetTargetLockWB _bpc_combat (Variables|/Game/ThirdPerson/Blueprints/BPC_Combat.BPC_Combat_C|GetTargetLockWB _bpc_combat))
  (Variables|/Script/Engine.CharacterMovementComponent|SetbOrientRotationToMovement _charactermovement true)
  (Variables|/Script/Engine.CharacterMovementComponent|SetbUseControllerDesiredRotation _charactermovement false)
  (Rendering|SetVisibility (Variables|Default|GetHealthBar) false false))

(event Game|Damage|EventAnyDamage
  (params (Damage :type Float%20%28single-precision%29) (DamageType :type Damage%20Type%20Object%20Reference) (InstigatedBy :type Controller%20Object%20Reference) (DamageCauser :type Actor%20Object%20Reference))
  (bind _charactermovement (Variables|Character|GetCharacterMovement))
  ;[0.15 0.15 0.15 0.5] Damage Received
  (Default|IncreaseValue (Variables|Default|GetBPC_Stats) "NewEnumerator0" (* Damage -1.0))
  (Animation|Montage|PlayMontage (Variables|Character|GetMesh) "/Game/Dark_Knight/Dark_Knight_Female/Animations/Anim_DKF_Hit_Fwd_Montage.Anim_DKF_Hit_Fwd_Montage"
    (:then
      (Variables|/Script/Engine.CharacterMovementComponent|SetMaxWalkSpeed _charactermovement 0.0))
    (:OnCompleted
      (Variables|/Script/Engine.CharacterMovementComponent|SetMaxWalkSpeed _charactermovement 4e+02 :!label _label))
    (:OnInterrupted
      (goto _label))))

(fn ConstructionScript)

(fn HardAttack
  (bind _returnvalue (Animation|PlayAnimMontage (Variables|Default|GetHardAttackMontage) 1.0 "None"))
  (return _returnvalue))

(fn SwordAttack
  (bind _returnvalue (Animation|PlayAnimMontage (Variables|Default|GetSwordAttackMontage) 1.0 "None"))
  (return _returnvalue))